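; Cart actor that rides along the spline of a referenced track actor, starting on BeginPlay when ActiveCart is set.
; The CartMover timeline starts from CartStartOffset, with its play rate set to the inverse of Duration.
; Each update maps the timeline Alpha to a distance along the spline and applies that point's world location and rotation to the cart.
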(event `self.ReceiveBeginPlay`
  (if (`self.ActiveCart`)
    (`self.MoveCart`)))

(event `MoveCart`
  (bind _cartmover (`self.CartMover`))
  (bind _usefulspline (`/Game/Blueprints/Track.UsefulSpline` (`self.TrackRef`)))
  (bind _returnvalue (`KismetMathLibrary.Lerp` 0.0 (`SplineComponent.GetSplineLength` _usefulspline) (`self.Alpha`)))
  (`TimelineComponent.SetPlayRate` _cartmover (/ 1.0 (`self.Duration`)))
  (`TimelineComponent.SetNewTime` _cartmover (`self.CartStartOffset`))
  (bind (_direction _alpha) (`Timeline|CartMover`)
    (:`Update`
      (set `self.Alpha` _alpha)
      (`self.K2_SetActorLocationAndRotation` (`SplineComponent.GetLocationAtDistanceAlongSpline` _usefulspline _returnvalue "World") (`SplineComponent.GetRotationAtDistanceAlongSpline` _usefulspline _returnvalue "World")))))

(event `self.ReceiveTick`
  (params (DeltaSeconds :type "Float (single-precision)")))

(fn `UserConstructionScript`)
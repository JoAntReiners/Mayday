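; Player character for an auto-forward flying shooter, handling steering, dodges, shooting, health and level restart.
; Tick drives forward movement and delayed passive health drain, while steering and dodge launches clamp position to Y/Z bounds and dodges share a global cooldown.
; A gate-and-delay loop repeats laser fire while held; weapon cycling only updates GunMode.
; Pickups heal, collisions damage then grant brief invulnerability, and death only prints a message.
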(event `self.ReceiveBeginPlay`
  ;[1 1 1] Initialize HUD
  (`self.InitializeHUD`))

(event `InputAction|TempRestart`
  (params (Key :type "Key Structure"))
  ;[1 1 1] TempRestart
  (:`Pressed`
    (`self.RestartLevel`)))

(event `InputAction|Fire`
  (params (Key :type "Key Structure"))
  ;[1 1 1] Combat
  ;;[1 1 1] Fire Bullets
  (:`Pressed`
    (`|ExecutionSequence`
      (:`then_0`
        (goto _label :!via `Open`))
      (:`then_1`
        (`/Engine/EditorBlueprintResources/StandardMacros.Gate` true :!label _label
          (:`Exit`
            (`self.FireGun`)
            (`KismetSystemLibrary.Delay` 0.2)
            (goto _label))))))
  (:`Released`
    (goto _label :!via `Close`)))

(event `InputAxis|CycleWeapons`
  (params (AxisValue :type "Float (single-precision)"))
  ;[1 1 1] Combat
  ;;[1 1 1] Cycle Weapon
  (`self.UpdateWeapon` AxisValue))

(event `self.ReceiveActorBeginOverlap`
  (params (OtherActor :type "Actor Object Reference"))
  ;[1 1 1] Combat
  ;;[1 1 1] Player Collision
  (if (`self.ActorHasTag` OtherActor "Pickup")
    (`self.ExecuteHealthPIckup` OtherActor)
    (elif (`self.ActorHasTag` OtherActor "Enemy")
      (`self.K2_DestroyActor` OtherActor)
      (bind _isdead (`self.CheckInvuln`))
      (if _isdead
        (`KismetSystemLibrary.PrintString` "You Died!" true true (struct :`R` 0.734375 :`G` 0.375375 :`A` 1.0) 5.0)
        (else
          (`KismetSystemLibrary.Delay` 3.0)
          (set `self.Invuln` false))))))

(event `self.ReceiveHit`
  (params (MyComp :type "PrimitiveComponent Object Reference") (Other :type "Actor Object Reference") (OtherComp :type "PrimitiveComponent Object Reference") (bSelfMoved :type Boolean) (HitLocation :type "Vector Structure") (HitNormal :type "Vector Structure") (NormalImpulse :type "Vector Structure") (Hit :type "HitResult Structure (by ref)"))
  ;[1 1 1] Combat
  ;;[1 1 1] Player Collision
  (bind _isdead (`self.CheckInvuln`))
  (if _isdead
    (`KismetSystemLibrary.PrintString` "You Died!" true true (struct :`R` 0.734375 :`G` 0.375375 :`A` 1.0) 5.0)
    (else
      (`KismetSystemLibrary.Delay` 3.0)
      (set `self.Invuln` false))))

(event `self.ReceiveTick`
  (params (DeltaSeconds :type "Float (single-precision)"))
  ;[1 1 1] Movement
  ;;[1 1 1] Basic Movement
  (`|ExecutionSequence`
    (:`then_0`
      (`self.BasicMovement` (`self.GetActorForwardVector`) (`self.Speed`)))
    (:`then_1`
      (`KismetSystemLibrary.Delay` (`self.HealthLossRate`))
      (`self.DeincrementHealth`))))

(event `InputAction|DodgeRight`
  (params (Key :type "Key Structure"))
  ;[1 1 1] Movement
  ;;[1 1 1] Advanced Movement
  (:`Pressed`
    (`/Engine/EditorBlueprintResources/StandardMacros.CompareFloat` (`self.GlobalCoolDown`) (`KismetSystemLibrary.GetGameTimeInSeconds`)
      (:`<`
        (`self.Dodge` (* (`self.GetActorRightVector`) (`self.DodgeSpeedHorizontal`)))
        (`KismetSystemLibrary.Delay` 0.2)
        (`self.ResumeNormalMovement` (`self.CharacterMovement`))))))

(event `InputAxis|Horizontal`
  (params (AxisValue :type "Float (single-precision)"))
  ;[1 1 1] Movement
  ;;[1 1 1] Basic Movement
  (`self.BasicMovement` (`self.GetActorRightVector`) AxisValue))

(event `InputAxis|Vertical`
  (params (AxisValue :type "Float (single-precision)"))
  ;[1 1 1] Movement
  ;;[1 1 1] Basic Movement
  (`self.BasicMovement` (`self.GetActorUpVector`) AxisValue))

(event `InputAction|DodgeLeft`
  (params (Key :type "Key Structure"))
  ;[1 1 1] Movement
  ;;[1 1 1] Advanced Movement
  (:`Pressed`
    (`/Engine/EditorBlueprintResources/StandardMacros.CompareFloat` (`self.GlobalCoolDown`) (`KismetSystemLibrary.GetGameTimeInSeconds`)
      (:`<`
        (`self.Dodge` (* (`self.GetActorRightVector`) (* -1 (`self.DodgeSpeedHorizontal`))))
        (`KismetSystemLibrary.Delay` 0.2)
        (`self.ResumeNormalMovement` (`self.CharacterMovement`))))))

(event `InputAction|DodgeUp`
  (params (Key :type "Key Structure"))
  ;[1 1 1] Movement
  ;;[1 1 1] Advanced Movement
  (:`Pressed`
    (`/Engine/EditorBlueprintResources/StandardMacros.CompareFloat` (`self.GlobalCoolDown`) (`KismetSystemLibrary.GetGameTimeInSeconds`)
      (:`<`
        (`self.Dodge` (* (`self.GetActorUpVector`) (`self.DodgeSpeedVertical`)))
        (`KismetSystemLibrary.Delay` 0.2)
        (`self.ResumeNormalMovement` (`self.CharacterMovement`))))))

(event `InputAction|AirBrake`
  (params (Key :type "Key Structure"))
  ;[1 1 1] Movement
  ;;[1 1 1] Advanced Movement
  (:`Pressed`
    (`/Engine/EditorBlueprintResources/StandardMacros.CompareFloat` (`self.GlobalCoolDown`) (`KismetSystemLibrary.GetGameTimeInSeconds`)
      (:`<`
        (`self.Dodge` (* (`self.GetActorForwardVector`) (* -1 (`self.AirbrakeSpeed`))))
        (`KismetSystemLibrary.Delay` 0.2)
        (`self.ResumeNormalMovement` (`self.CharacterMovement`))))))

(fn `BasicMovement`
  (params (`World Direction` :type "Vector Structure") (`Scale Value` :type "Float (double-precision)"))
  (`self.AddMovementInput` `World Direction` `Scale Value`)
  (bind _clampedlocation (`self.GetClampedLocation`))
  (`self.K2_SetActorLocation` _clampedlocation))

(fn `CheckInvuln`
  (returns (isDead :type Boolean))
  (bind _health (`self.Health`))
  (bind _collisiondamage (`self.CollisionDamage`))
  (if (`self.Invuln`)
    (`KismetSystemLibrary.PrintString` "Player Invuln!" true true (struct :`G` 1.0 :`B` 0.329394 :`A` 1.0) 5.0)
    (else
      (set `self.Health` (- _health _collisiondamage))
      (set `self.Invuln` true)
      (`KismetSystemLibrary.PrintString` (`KismetStringLibrary.Concat_StrStr` "You took " (`KismetStringLibrary.Conv_IntToString` _collisiondamage) " damage!" " You now have " (`KismetStringLibrary.Conv_IntToString` _health) " Health.") true true (struct :`R` 1.0 :`G` 0.110816 :`B` 0.061054 :`A` 1.0) 5.0)
      (return (<= _health 0)))))

(fn `DeincrementHealth`
  (bind _output_get (set `self.Health` (- (`self.Health`) (`self.PassiveHealthLoss`))))
  (if (<= _output_get 0)
    (`KismetSystemLibrary.PrintString` "You Died!" true true (struct :`R` 0.734375 :`G` 0.375375 :`A` 1.0) 5.0)))

(fn `Dodge`
  (params (LaunchVelocity :type "Vector Structure"))
  (`self.LaunchCharacter` LaunchVelocity)
  (bind _clampedlocation (`self.GetClampedLocation`))
  (`self.K2_SetActorLocation` _clampedlocation))

(fn `ExecuteHealthPIckup`
  (params (`Hit Actor` :type "Actor Object Reference"))
  (bind _health (`self.Health`))
  (bind _returnvalue (+ _health (`self.PickupHealth`)))
  (if (> _returnvalue 100)
    (set `self.Health` 100)
    (else
      (set `self.Health` _returnvalue)))
  (`self.K2_DestroyActor` `Hit Actor`)
  (`KismetSystemLibrary.PrintString` (`KismetStringLibrary.Concat_StrStr` "You healed up to " (`KismetStringLibrary.Conv_IntToString` _health) " Health.")))

(fn `FireGun`
  (`ShootBullet.ShootBullet` "/Game/Blueprints/Character/Laser.Laser_C" (+ (`self.K2_GetActorLocation`) (* (`self.GetActorForwardVector`) 200.0)) (`self.GetControlRotation`)))

(fn `GetClampedLocation`
  (returns (ClampedLocation :type "Vector Structure"))
  (return (`KismetMathLibrary.MakeVector` (.x (`self.K2_GetActorLocation`)) (`KismetMathLibrary.FClamp` (.y (`self.K2_GetActorLocation`)) (`self.YMin`) (`self.YMax`)) (`KismetMathLibrary.FClamp` (.z (`self.K2_GetActorLocation`)) (`self.ZMin`) (`self.ZMax`)))))

(fn `GetSpeed`
  (params (GetSpeed :type "Float (double-precision)"))
  (returns (Speed :type "Float (double-precision)"))
  (set `self.Speed` GetSpeed)
  (return GetSpeed))

(fn `InitializeHUD`
  (bind _returnvalue (`|CreateWidget` "/Game/Blueprints/Character/HUD.HUD_C" (`GameplayStatics.GetPlayerController` 0)))
  (bind _output_get (set `self.HUD` _returnvalue))
  (`UserWidget.AddToViewport` _output_get 0))

(fn `RestartLevel`
  (bind _returnvalue (`GameplayStatics.GetCurrentLevelName` true))
  (`GameplayStatics.OpenLevel` (`KismetStringLibrary.Conv_StringToName` _returnvalue)))

(fn `ResumeNormalMovement`
  (params (CharacterMovement :type "CharacterMovementComponent Object Reference"))
  (`CharacterMovementComponent.SetMovementMode` CharacterMovement "MOVE_Flying" 0)
  (`MovementComponent.StopMovementImmediately` CharacterMovement)
  (`CharacterMovementComponent.ClearAccumulatedForces` CharacterMovement)
  (`self.UpdateGCD`))

(fn `UpdateGCD`
  (set `self.GlobalCoolDown` (+ (`KismetSystemLibrary.GetGameTimeInSeconds`) (`self.GCDIncrement`))))

(fn `UpdateWeapon`
  (params (Cycle :type "Float (double-precision)"))
  (bind _returnvalue (+ (`KismetMathLibrary.FTrunc` Cycle) (`self.GunMode`)))
  (if (not (or (> _returnvalue (`self.MaxGuns`)) (< _returnvalue (`self.MinGuns`))))
    (set `self.GunMode` _returnvalue)))

(fn `UserConstructionScript`)
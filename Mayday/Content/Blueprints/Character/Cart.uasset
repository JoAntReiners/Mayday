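; Cart actor meant to ride a track's spline, with its movement logic currently disconnected from BeginPlay and MoveCart.
; The unwired chains find the CartChara, start MoveCart if active, and drive a duration-scaled, offset timeline.
; Each timeline update would send CartChara a zero speed message and set location and rotation by distance along TrackRef's spline.
; GetSpeed is a stub returning zero.
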(event `self.ReceiveBeginPlay`
  ;[1 1 1] Initiallize Cart
)

(event `MoveCart`
  ;[1 1 1] Move Cart Along Spline
)

(fn `GetSpeed`
  (params (GetSpeed :type "Float (double-precision)"))
  (returns (Speed :type "Float (double-precision)"))
  (return 0.0))

(fn `UserConstructionScript`)
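; GatlingLaser is a short-lived projectile that damages enemies, destroying itself one second after spawning or on any hit or overlap.
; Overlaps run CheckHit, which filters for Enemy or Destructable tags, then subtracts BulletDamage from Health only if the actor casts to Enemy.
; An enemy whose Health reaches zero or below is destroyed, while Destructable actors of other classes take no damage.
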(event `self.ReceiveBeginPlay`
  (`KismetSystemLibrary.Delay` 1.0)
  (`self.K2_DestroyActor`))

(event `self.ReceiveActorBeginOverlap`
  (params (OtherActor :type "Actor Object Reference"))
  (`self.CheckHit` OtherActor))

(event `self.ReceiveHit`
  (params (MyComp :type "PrimitiveComponent Object Reference") (Other :type "Actor Object Reference") (OtherComp :type "PrimitiveComponent Object Reference") (bSelfMoved :type Boolean) (HitLocation :type "Vector Structure") (HitNormal :type "Vector Structure") (NormalImpulse :type "Vector Structure") (Hit :type "HitResult Structure (by ref)"))
  (`self.K2_DestroyActor`))

(fn `CheckHit`
  (params (Other :type "Actor Object Reference"))
  (`KismetSystemLibrary.PrintString` "Hit something")
  (if (or (`self.ActorHasTag` Other "Enemy") (`self.ActorHasTag` Other "Destructable"))
    (`self.K2_DestroyActor`)
    (bind _asenemy (cast `/Game/Blueprints/Enemy/Enemy` Other))
    (bind _output_get (set `/Game/Blueprints/Enemy/Enemy.Health` (- (`/Game/Blueprints/Enemy/Enemy.Health` _asenemy) (`self.BulletDamage`)) _asenemy))
    (`KismetSystemLibrary.PrintString` (`KismetStringLibrary.Conv_DoubleToString` _output_get))
    (if (<= _output_get 0.0)
      (`self.K2_DestroyActor` Other))
    (else
      (`self.K2_DestroyActor`))))

(fn `UserConstructionScript`)
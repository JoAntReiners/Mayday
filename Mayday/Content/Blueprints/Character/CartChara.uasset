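; Player character for an auto-forward flying shooter, steered within Y and Z limits and firing lasers along control rotation.
; Tick drives forward movement at Speed and, through a Delay, periodic passive health drain; death only prints a message.
; Pickups restore health up to a cap, while hits and other overlaps deal damage followed by brief invulnerability.
; It also creates the HUD and offers a temporary level-restart input; GetSpeed actually sets Speed.
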(event `InputAction|TempRestart`
  (params (Key :type "Key Structure"))
  (:`Pressed`
    (bind _returnvalue (`GameplayStatics.GetCurrentLevelName` true))
    (`GameplayStatics.OpenLevel` (`KismetStringLibrary.Conv_StringToName` _returnvalue))))

(event `self.ReceiveBeginPlay`
  ;[1 1 1] Initialize HUD
  (bind _returnvalue (`|CreateWidget` "/Game/Blueprints/Character/HUD.HUD_C" (`GameplayStatics.GetPlayerController` 0)))
  (bind _output_get (set `self.HUD` _returnvalue))
  (`UserWidget.AddToViewport` _output_get 0))

(event `self.ReceiveTick`
  (params (DeltaSeconds :type "Float (single-precision)"))
  ;[1 1 1] Plane Movement
  (`|ExecutionSequence`
    (:`then_0`
      (`self.AddMovementInput` (`self.GetActorForwardVector`) (`self.Speed`)))
    (:`then_1`
      (`KismetSystemLibrary.Delay` (`self.HealthLossRate`))
      (bind _output_get (set `self.Health` (- (`self.Health`) (`self.PassiveHealthLoss`))))
      (if (<= _output_get 0)
        (`KismetSystemLibrary.PrintString` "You Died!" true true (struct :`R` 0.734375 :`G` 0.375375 :`A` 1.0) 5.0)))))

(event `InputAction|Fire`
  (params (Key :type "Key Structure"))
  ;[1 1 1] Fire Bullets
  (:`Pressed`
    (`ShootBullet.ShootBullet` "/Game/Blueprints/Character/Laser.Laser_C" (+ (`self.K2_GetActorLocation`) (* (`self.GetActorForwardVector`) 200.0)) (`self.GetControlRotation`))))

(event `self.ReceiveActorBeginOverlap`
  (params (OtherActor :type "Actor Object Reference"))
  (bind _health (`self.Health`))
  (bind _health_2 (`self.Health`))
  (bind _collisiondamage (`self.CollisionDamage`))
  (bind _returnvalue (+ _health_2 (`self.PickupHealth`)))
  ;[1 1 1] Player Collision
  (if (`self.ActorHasTag` OtherActor "Pickup")
    (if (> _returnvalue 100)
      (set `self.Health` 100)
      (else
        (set `self.Health` _returnvalue)))
    (`self.K2_DestroyActor` OtherActor)
    (`KismetSystemLibrary.PrintString` (`KismetStringLibrary.Concat_StrStr` "You healed up to " (`KismetStringLibrary.Conv_IntToString` _health_2) " Health."))
    (else
      (if (`self.ActorHasTag` OtherActor "Enemy")
        (`self.K2_DestroyActor` OtherActor))
      (if (`self.Invuln`)
        (`KismetSystemLibrary.PrintString` "Player Invuln!" true true (struct :`G` 1.0 :`B` 0.329394 :`A` 1.0) 5.0)
        (else
          (set `self.Health` (- _health _collisiondamage))
          (set `self.Invuln` true)
          (`KismetSystemLibrary.PrintString` (`KismetStringLibrary.Concat_StrStr` "You took " (`KismetStringLibrary.Conv_IntToString` _collisiondamage) " damage!" " You now have " (`KismetStringLibrary.Conv_IntToString` _health) " Health.") true true (struct :`R` 1.0 :`G` 0.110816 :`B` 0.061054 :`A` 1.0) 5.0)
          (if (<= _health 0)
            (`KismetSystemLibrary.PrintString` "You Died!" true true (struct :`R` 0.734375 :`G` 0.375375 :`A` 1.0) 5.0)
            (else
              (`KismetSystemLibrary.Delay` 3.0)
              (set `self.Invuln` false))))))))

(event `InputAxis|Horizontal`
  (params (AxisValue :type "Float (single-precision)"))
  (bind _y (.y (`self.K2_GetActorLocation`)))
  ;[1 1 1] Plane Movement
  (if (> AxisValue 0.0)
    (if (< _y (`self.YMax`))
      (`self.AddMovementInput` (`self.GetActorRightVector`) AxisValue :!label _label))
    (elif (> _y (`self.YMin`))
      (goto _label))))

(event `InputAxis|Vertical`
  (params (AxisValue :type "Float (single-precision)"))
  (bind _z (.z (`self.K2_GetActorLocation`)))
  ;[1 1 1] Plane Movement
  (if (> AxisValue 0.0)
    (if (< _z (`self.ZMax`))
      (`self.AddMovementInput` (`self.GetActorUpVector`) AxisValue :!label _label_2))
    (elif (> _z (`self.ZMin`))
      (goto _label_2))))

(event `self.ReceiveHit`
  (params (MyComp :type "PrimitiveComponent Object Reference") (Other :type "Actor Object Reference") (OtherComp :type "PrimitiveComponent Object Reference") (bSelfMoved :type Boolean) (HitLocation :type "Vector Structure") (HitNormal :type "Vector Structure") (NormalImpulse :type "Vector Structure") (Hit :type "HitResult Structure (by ref)"))
  (bind _health (`self.Health`))
  (bind _collisiondamage (`self.CollisionDamage`))
  ;[1 1 1] Player Collision
  (if (`self.Invuln`)
    (`KismetSystemLibrary.PrintString` "Player Invuln!" true true (struct :`G` 1.0 :`B` 0.329394 :`A` 1.0) 5.0)
    (else
      (set `self.Health` (- _health _collisiondamage))
      (set `self.Invuln` true)
      (`KismetSystemLibrary.PrintString` (`KismetStringLibrary.Concat_StrStr` "You took " (`KismetStringLibrary.Conv_IntToString` _collisiondamage) " damage!" " You now have " (`KismetStringLibrary.Conv_IntToString` _health) " Health.") true true (struct :`R` 1.0 :`G` 0.110816 :`B` 0.061054 :`A` 1.0) 5.0)
      (if (<= _health 0)
        (`KismetSystemLibrary.PrintString` "You Died!" true true (struct :`R` 0.734375 :`G` 0.375375 :`A` 1.0) 5.0)
        (else
          (`KismetSystemLibrary.Delay` 3.0)
          (set `self.Invuln` false))))))

(fn `GetSpeed`
  (params (GetSpeed :type "Float (double-precision)"))
  (returns (Speed :type "Float (double-precision)"))
  (set `self.Speed` GetSpeed)
  (return GetSpeed))

(fn `UserConstructionScript`)